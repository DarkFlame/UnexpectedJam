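; Generator Blueprint that plays a scripted power sound sequence when its Trigger event fires.
; Trigger spawns the Lights 2D sound six times with mostly shortening delays, then after a longer pause plays the Generator 2D sound.
; Timing is a hard-coded chain of Delay nodes; BeginPlay, overlap and Tick are disabled, and the construction script only calls its parent.
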(event `/Game/Blueprints/BaseClasses/Triggerable.Trigger`
  (`GameplayStatics.SpawnSound2D` "/Game/Audio/Lights.Lights" 1.0 1.0 0.0 null)
  (`KismetSystemLibrary.Delay` 1.0)
  (`GameplayStatics.SpawnSound2D` "/Game/Audio/Lights.Lights" 1.0 1.0 0.0 null)
  (`KismetSystemLibrary.Delay` 1.0)
  (`GameplayStatics.SpawnSound2D` "/Game/Audio/Lights.Lights" 1.0 1.0 0.0 null)
  (`KismetSystemLibrary.Delay` 0.5)
  (`GameplayStatics.SpawnSound2D` "/Game/Audio/Lights.Lights" 1.0 1.0 0.0 null)
  (`KismetSystemLibrary.Delay` 0.5)
  (`GameplayStatics.SpawnSound2D` "/Game/Audio/Lights.Lights" 1.0 1.0 0.0 null)
  (`KismetSystemLibrary.Delay` 0.4)
  (`GameplayStatics.SpawnSound2D` "/Game/Audio/Lights.Lights" 1.0 1.0 0.0 null)
  (`KismetSystemLibrary.Delay` 0.3)
  (`GameplayStatics.SpawnSound2D` "/Game/Audio/Lights.Lights" 1.0 1.0 0.0 null)
  (`KismetSystemLibrary.Delay` 2.0)
  (`GameplayStatics.PlaySound2D` "/Game/Audio/Generator.Generator" 1.0 1.0 0.0 null null))

(fn `UserConstructionScript`
  (`parent.UserConstructionScript`))