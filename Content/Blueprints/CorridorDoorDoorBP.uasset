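; CorridorDoorDoorBP is a corridor door that opens for the player only while the power is on.
; BeginPlay caches the game state, whose LightsOn flag gates both overlap events and prints "Power not on" when false.
; Player overlap plays the Dooropening timeline to move the door mesh along local Z, and leaving reverses it.
; Open and Close snap the door along Y but are never run.
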(event `self.ReceiveBeginPlay`
  (bind _as_game_state_unexpected (cast `/Game/Blueprints/_GameStateUnexpected` (`GameplayStatics.GetGameState`)))
  (set `self.State` _as_game_state_unexpected))

(event `self.ReceiveActorBeginOverlap`
  (params (OtherActor :type "Actor Object Reference"))
  (if (`/Game/Blueprints/_GameStateUnexpected.Lights_on` (`self.State`))
    (if (== OtherActor (`GameplayStatics.GetPlayerCharacter` 0))
      (bind (_direction _offset) (`Timeline|Dooropening` :!label _label)
        (:`Update`
          (`SceneComponent.K2_SetRelativeLocation` (`self.CorridorDoorDoor`) (`KismetMathLibrary.MakeVector` 0.0 0.0 _offset) false false))))
    (else
      (`KismetSystemLibrary.PrintString` "Power not on"))))

(event `self.ReceiveActorEndOverlap`
  (params (OtherActor :type "Actor Object Reference"))
  (if (`/Game/Blueprints/_GameStateUnexpected.Lights_on` (`self.State`))
    (if (== OtherActor (`GameplayStatics.GetPlayerCharacter` 0))
      (goto _label :!via `Reverse`))
    (else
      (`KismetSystemLibrary.PrintString` "Power not on"))))

(fn `Close`
  (`SceneComponent.K2_SetRelativeLocation` (`self.CorridorDoorDoor`) (0.0 0.0 0.0) false false))

(fn `Open`
  (`SceneComponent.K2_SetRelativeLocation` (`self.CorridorDoorDoor`) (0.0 250.0 0.0) false false))

(fn `UserConstructionScript`)