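; Interactable child Blueprint for the information sorting step, which responds to Trigger with dialog driven by WorldState flags.
; It plays a bad beep until the world is Stabilized, then the first trigger sets InformationSorted and later triggers report it running.
; InterpreterOn selects readable text, with the first message flagged as a question, or the same lines with their letters sorted alphabetically.
; The parent Trigger runs after each dialog is set.
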(event `self.Trigger`
  (if (`/Game/Blueprints/_GameStateUnexpected.Information_Sorted` (`self.WorldState`))
    (if (`/Game/Blueprints/_GameStateUnexpected.Interpreter_On` (`self.WorldState`))
      (`self.SetDialog` "Information sorting active and running.")
      (`self.SetIsQuestion` false)
      (`parent.Trigger`)
      (else
        (`self.SetDialog` "aaa c d e f gg iiiii m nnnnnnn ooo rrr s ttt u v .")
        (`self.SetIsQuestion` false)
        (`parent.Trigger`)))
    (elif (`/Game/Blueprints/_GameStateUnexpected.Stabilized` (`self.WorldState`))
      (if (`/Game/Blueprints/_GameStateUnexpected.Interpreter_On` (`self.WorldState`))
        (set `/Game/Blueprints/_GameStateUnexpected.Information_Sorted` true (`self.WorldState`))
        (`self.SetDialog` "Hello? Can you understand me?")
        (`self.SetIsQuestion` true)
        (`parent.Trigger`)
        (else
          (`self.SetDialog` "aaaa cc ee f hh i n oooo rr s tt uuu ww yy.??")
          (`self.SetIsQuestion` false)
          (set `/Game/Blueprints/_GameStateUnexpected.Information_Sorted` true (`self.WorldState`))
          (`parent.Trigger`)))
      (else
        (`GameplayStatics.PlaySound2D` "/Game/Audio/Badbeep.Badbeep" 1.0 1.0 0.0 null null)))))

(fn `UserConstructionScript`
  (`parent.UserConstructionScript`))