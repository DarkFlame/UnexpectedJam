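; Base dialog trigger that opens a dialog box, either plain or flagged as a question, when its Trigger event fires.
; It passes its dialog text, question flag and two buttons, each built from a text and response pair, to WorldState to create the box.
; It then switches the first player controller to UI-only input without locking the mouse.
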(event `self.Trigger`
  (`/Game/Blueprints/BaseClasses/GameStateUnexpected.CreateDialogBox` (`self.WorldState`) (`self.Dialog`) 0.05 (`self.isQuestion`) (make `/Game/Blueprints/BaseClasses/Button` (`self.Button1 Text`) (`self.Button1 Response`)) (make `/Game/Blueprints/BaseClasses/Button` (`self.Button2 Text`) (`self.Button2 Response`)))
  (`WidgetBlueprintLibrary.SetInputMode_UIOnlyEx` (`GameplayStatics.GetPlayerController` 0) null))

(fn `UserConstructionScript`
  (`parent.UserConstructionScript`))