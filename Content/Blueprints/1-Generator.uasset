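; Generator Blueprint that powers up seven lights in sequence when its Trigger event fires.
; It first sets the LightsOn flag on WorldState, then plays a 2D sound as each light is raised to LightIntensity through the TurnOnALight helper.
; Hard-coded delays shorten along the chain so the lights come on faster, and after a final pause the generator sound plays.
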(event `self.Trigger`
  (set `/Game/Blueprints/_GameStateUnexpected.Lights_on` true (`self.WorldState`))
  (`GameplayStatics.SpawnSound2D` "/Game/Audio/Lights.Lights" 1.0 1.0 0.0 null)
  (`self.TurnOnALight` (`self.Light_0`))
  (`KismetSystemLibrary.Delay` 1.0)
  (`GameplayStatics.SpawnSound2D` "/Game/Audio/Lights.Lights" 1.0 1.0 0.0 null)
  (`self.TurnOnALight` (`self.Light_1`))
  (`KismetSystemLibrary.Delay` 1.0)
  (`GameplayStatics.SpawnSound2D` "/Game/Audio/Lights.Lights" 1.0 1.0 0.0 null)
  (`self.TurnOnALight` (`self.Light_2`))
  (`KismetSystemLibrary.Delay` 0.5)
  (`GameplayStatics.SpawnSound2D` "/Game/Audio/Lights.Lights" 1.0 1.0 0.0 null)
  (`self.TurnOnALight` (`self.Light_3`))
  (`KismetSystemLibrary.Delay` 0.5)
  (`GameplayStatics.SpawnSound2D` "/Game/Audio/Lights.Lights" 1.0 1.0 0.0 null)
  (`self.TurnOnALight` (`self.Light_4`))
  (`KismetSystemLibrary.Delay` 0.4)
  (`GameplayStatics.SpawnSound2D` "/Game/Audio/Lights.Lights" 1.0 1.0 0.0 null)
  (`self.TurnOnALight` (`self.Light_5`))
  (`KismetSystemLibrary.Delay` 0.3)
  (`GameplayStatics.SpawnSound2D` "/Game/Audio/Lights.Lights" 1.0 1.0 0.0 null)
  (`self.TurnOnALight` (`self.Light_6`))
  (`KismetSystemLibrary.Delay` 2.0)
  (`GameplayStatics.PlaySound2D` "/Game/Audio/Generator.Generator" 1.0 1.0 0.0 null null))

(fn `TurnOnALight`
  (params (ALight :type "Light Object Reference"))
  (`LightComponent.SetIntensity` (`Light.LightComponent` ALight) (`self.Light Intensity`)))

(fn `UserConstructionScript`
  (`parent.UserConstructionScript`))