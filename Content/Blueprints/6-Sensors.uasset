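; Sensors switch interactable that shows AI dialogue and can switch on the sensors flag in WorldState.
; Trigger enables the sensors and plays an Eyeball sound only once Stabilized is set; otherwise the switch reports no response.
; InterpreterOn and InformationSorted select coherent, word-scrambled or silent "..." lines, both on activation and when already active.
; Each branch sets non-question dialogue and defers to the parent Trigger.
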(event `self.Trigger`
  (if (`/Game/Blueprints/_GameStateUnexpected.Sensors_On` (`self.WorldState`))
    (if (`/Game/Blueprints/_GameStateUnexpected.Interpreter_On` (`self.WorldState`))
      (if (`/Game/Blueprints/_GameStateUnexpected.Information_Sorted` (`self.WorldState`))
        (`self.SetDialog` "Sensors currently active. I can see you...")
        (`self.SetIsQuestion` false)
        (`parent.Trigger`)
        (else
          (`self.SetDialog` "Sensors I can you... active. see currently")
          (`self.SetIsQuestion` false)
          (`parent.Trigger`)))
      (else
        (`self.SetDialog` "...")
        (`self.SetIsQuestion` false)
        (`parent.Trigger`)))
    (elif (`/Game/Blueprints/_GameStateUnexpected.Stabilized` (`self.WorldState`))
      (if (`/Game/Blueprints/_GameStateUnexpected.Interpreter_On` (`self.WorldState`))
        (if (`/Game/Blueprints/_GameStateUnexpected.Information_Sorted` (`self.WorldState`))
          (set `/Game/Blueprints/_GameStateUnexpected.Sensors_On` true (`self.WorldState`))
          (`self.SetDialog` "There you are. You're smaller than I was expecting.")
          (`self.SetIsQuestion` false)
          (`parent.Trigger`)
          (`GameplayStatics.SpawnSound2D` "/Game/Audio/Eyeball.Eyeball" 1.0 1.0 0.0 null)
          (else
            (set `/Game/Blueprints/_GameStateUnexpected.Sensors_On` true (`self.WorldState`))
            (`self.SetDialog` "I was There smaller than expecting. You're you are.")
            (`self.SetIsQuestion` false)
            (`parent.Trigger`)
            (`GameplayStatics.SpawnSound2D` "/Game/Audio/Eyeball.Eyeball" 1.0 1.0 0.0 null)))
        (else
          (set `/Game/Blueprints/_GameStateUnexpected.Sensors_On` true (`self.WorldState`))
          (`self.SetDialog` "...")
          (`self.SetIsQuestion` false)
          (`parent.Trigger`)
          (`GameplayStatics.SpawnSound2D` "/Game/Audio/Eyeball.Eyeball" 1.0 1.0 0.0 null)))
      (else
        (`self.SetDialog` "[The switch does not respond...]")
        (`self.SetIsQuestion` false)
        (`parent.Trigger`)))))

(fn `UserConstructionScript`
  (`parent.UserConstructionScript`))