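; Base dialog trigger Blueprint that opens an in-game dialog box, optionally as a question with two response buttons.
; Trigger passes the stored text, question flag and button structs to WorldState.CreateDialogBox, then switches the player controller to UI-only input.
; SetDialog updates the text at runtime.
; SetButton1 writes to the Button2 variables, while SetButton2 is empty.
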(event `self.Trigger`
  (`/Game/Blueprints/_GameStateUnexpected.CreateDialogBox` (`self.WorldState`) (`self.Dialog`) 0.05 (`self.isQuestion`) (make `/Game/Blueprints/Struct_Button` (`self.Button1 Text`) (`self.Button1 Response`)) (make `/Game/Blueprints/Struct_Button` (`self.Button2 Text`) (`self.Button2 Response`)))
  (`WidgetBlueprintLibrary.SetInputMode_UIOnlyEx` (`GameplayStatics.GetPlayerController` 0) null))

(fn `SetButton1`
  (params (Text :type Text) (Response :type Text))
  (set `self.Button2 Text` Text)
  (set `self.Button2 Response` Response))

(fn `SetButton2`
  (params (Text :type Text) (Response :type Text)))

(fn `SetDialog`
  (params (NewParam :type Text))
  (set `self.Dialog` NewParam))

(fn `UserConstructionScript`
  (`parent.UserConstructionScript`))