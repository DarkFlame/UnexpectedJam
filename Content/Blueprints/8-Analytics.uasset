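; Analytics interactable Blueprint whose Trigger event delivers the closing dialog and ends the game.
; When WorldState reports the databanks are on, it shows a farewell line, calls the parent trigger, waits, fades the camera and audio, then calls EndGame.
; Otherwise it shows a no-response line and still runs the parent trigger.
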(event `self.Trigger`
  (if (`/Game/Blueprints/_GameStateUnexpected.Databanks_On` (`self.WorldState`))
    (`self.SetDialog` "Maintenence check complete, all systems are operational. \nSo, what now? Are you going to leave me here, alone, like everyone else?")
    (`parent.Trigger`)
    (`KismetSystemLibrary.Delay` 30.0)
    (`PlayerCameraManager.StartCameraFade` :`self` (`GameplayStatics.GetPlayerCameraManager` 0) :`FromAlpha` 1.0 :`Duration` 2.0 :`bShouldFadeAudio` true :`bHoldWhenFinished` true)
    (`/Game/Blueprints/_GameStateUnexpected.EndGame` (`self.WorldState`))
    (else
      (`self.SetDialog` "[There is no response]")
      (`parent.Trigger`))))

(fn `UserConstructionScript`
  (`parent.UserConstructionScript`))