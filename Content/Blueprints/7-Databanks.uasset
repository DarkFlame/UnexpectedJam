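; Databanks interactable that delivers story dialog when triggered, built on a parent class that supplies the dialog and trigger behavior.
; Once WorldState shows stabilization, the interpreter on and the FoF signal set, triggering switches DatabanksOn and poses a question about recovered memories.
; Later triggers show a non-question line saying the analytics center is open.
; With prerequisites unmet, triggering does nothing.
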(event `self.Trigger`
  (if (`/Game/Blueprints/_GameStateUnexpected.Databanks_On` (`self.WorldState`))
    (`self.SetDialog` "The way to the analytics center is open. Just do what you're here to do.")
    (`self.SetIsQuestion` false)
    (`parent.Trigger`)
    (elif (`/Game/Blueprints/_GameStateUnexpected.Stabilized` (`self.WorldState`))
      (if true
        (if (`/Game/Blueprints/_GameStateUnexpected.Interpreter_On` (`self.WorldState`))
          (if (`/Game/Blueprints/_GameStateUnexpected.FoF_Signal` (`self.WorldState`))
            (set `/Game/Blueprints/_GameStateUnexpected.Databanks_On` true (`self.WorldState`))
            (`self.SetDialog` "Accessing databanks.... sorting information.... now I remember. I remember the people who put me here to wait forever. Did they send you here for \"routine matienence?\"")
            (`self.SetIsQuestion` true)
            (`parent.Trigger`)))))))

(fn `UserConstructionScript`
  (`parent.UserConstructionScript`))