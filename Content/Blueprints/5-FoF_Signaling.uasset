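; FoF signaling interactable that picks a line of dialog when triggered, based on world state.
; Trigger does nothing unless the world state is Stabilized, then branches on InterpreterOn and InformationSorted before calling the parent Trigger.
; With both set, it raises FoFSignal and asks a question; otherwise it gives a hostile warning or a scream.
; The inner InterpreterOn check is redundant, so the word-scrambled warning is unreachable.
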(event `self.Trigger`
  (if (`/Game/Blueprints/_GameStateUnexpected.Stabilized` (`self.WorldState`))
    (if (`/Game/Blueprints/_GameStateUnexpected.Interpreter_On` (`self.WorldState`))
      (if (`/Game/Blueprints/_GameStateUnexpected.Information_Sorted` (`self.WorldState`))
        (set `/Game/Blueprints/_GameStateUnexpected.FoF_Signal` true (`self.WorldState`))
        (`self.SetDialog` "Hello? Can you understand me?")
        (`self.SetIsQuestion` true)
        (`parent.Trigger`)
        (elif (`/Game/Blueprints/_GameStateUnexpected.Interpreter_On` (`self.WorldState`))
          (`self.SetDialog` "STAY AWAY! YOU CAN'T BE TRUSTED!")
          (`self.SetIsQuestion` false)
          (`parent.Trigger`)
          (else
            (`self.SetDialog` "TRUSTED! BE CAN'T YOU STAY AWAY!")
            (`self.SetIsQuestion` false)
            (`parent.Trigger`))))
      (else
        (`self.SetDialog` "Aaaaaaaaaaaaaaaaaaaaaaaaaaowowowowowowow")
        (`self.SetIsQuestion` false)
        (`parent.Trigger`)))))

(fn `UserConstructionScript`
  (`parent.UserConstructionScript`))